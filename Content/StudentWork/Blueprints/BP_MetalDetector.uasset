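; Metal detector actor that flashes a red alert whenever any actor overlaps it.
; Begin overlap sets an Activated flag, and end overlap clears it after a short delay.
; While active, Tick drives a FlipFlop into two delayed branches that swap two mesh material slots between emissive red and the sci-fi material.
; When inactive, Tick feeds the delayed sci-fi material branch directly.
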(event `self.ReceiveActorBeginOverlap`
  (params (OtherActor :type "Actor Object Reference"))
  ;[0 1 0.9508] Alert
  (set `self.Activated` true))

(event `self.ReceiveActorEndOverlap`
  (params (OtherActor :type "Actor Object Reference"))
  ;[0 1 0.9508] Alert
  (`KismetSystemLibrary.Delay` 5.0)
  (set `self.Activated` false))

(event `self.ReceiveTick`
  (params (DeltaSeconds :type "Float (single-precision)"))
  (bind _sm_metaldetector (`self.SM_MetalDetector`))
  (bind _sm_metaldetector_2 (`self.SM_MetalDetector`))
  ;[0 1 0.9508] Alert
  (if (== (`self.Activated`) true)
    (`/Engine/EditorBlueprintResources/StandardMacros.FlipFlop`
      (:`A`
        (`KismetSystemLibrary.Delay` 1.0)
        (`PrimitiveComponent.SetMaterial` _sm_metaldetector_2 2 "/Game/Materials/MI_EmissiveRed.MI_EmissiveRed")
        (`PrimitiveComponent.SetMaterial` _sm_metaldetector_2 4 "/Game/Materials/MI_EmissiveRed.MI_EmissiveRed"))
      (:`B`
        (`KismetSystemLibrary.Delay` 1.0 :!label _label)
        (`PrimitiveComponent.SetMaterial` _sm_metaldetector 2 "/Game/Materials/MI_SciFi_7.MI_SciFi_7")
        (`PrimitiveComponent.SetMaterial` _sm_metaldetector 4 "/Game/Materials/MI_SciFi_7.MI_SciFi_7")))
    (else
      (goto _label))))

(fn `UserConstructionScript`)