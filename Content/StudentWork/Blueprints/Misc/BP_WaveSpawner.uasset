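; Wave spawner that starts enemy waves by queuing enemies on the level's BP_Spawner actors.
; A looping timer checks whether no enemies remain, then gathers spawners, sets a cooldown timer and starts the wave immediately.
; StartWave totals the EnemyPool map into EnemyRemaining and queues a capped number on random spawners.
; Work in progress: every enemy is BP_Enemy_Chaser and EndWave is empty.
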(event `self.ReceiveBeginPlay`
  (`KismetSystemLibrary.K2_SetTimerDelegate` (delegate `TrySpawning`) 2.0 true))

(event `TrySpawning`
  (if (<= (`self.EnemyRemaining`) 0)
    (`self.Get Spawners`)
    (`self.EnterTransition`)))

(fn `BuildEnemyPool`
  (locals (LocalSum :type Integer))
  (set `self.EnemyRemaining` (`self.GetPoolSize`)))

(fn `End Wave`)

(fn `EnterTransition`
  (set `self.WaveCooldown` false)
  (`KismetSystemLibrary.K2_SetTimerDelegate` (`|CreateDelegate` :!event `Start Wave`) 20.0)
  (set `self.WaveCooldown` false)
  (`self.Start Wave`))

(fn `Get Spawners`
  (bind _outactors (`GameplayStatics.GetAllActorsOfClass` "/Game/StudentWork/Blueprints/Enemies/BP_Spawner.BP_Spawner_C"))
  (set `self.Spawners` _outactors))

(fn `GetEnemyFromPool`
  (returns (`Enemy Class` :type "/Game/StudentWork/Blueprints/Enemies/BP_Enemy_Chaser Class Reference"))
  (return "/Game/StudentWork/Blueprints/Enemies/BP_Enemy_Chaser.BP_Enemy_Chaser_C"))

(fn `GetPoolSize`
  (returns (Sum :type Integer))
  (locals (LocalTotal :type Integer))
  (bind _values (`BlueprintMapLibrary.Map_Values` (`self.EnemyPool`)))
  (for _array_element _values
    (set `local.LocalTotal` (+ _array_element (`local.LocalTotal`))))
  (return (`local.LocalTotal`)))

(fn `NewWave`
  (`/Engine/EditorBlueprintResources/StandardMacros.IncrementInt` (`self.WaveNumber`)
    (:`  `
      (`self.Start Wave`))))

(fn `Start Wave`
  (`self.BuildEnemyPool`)
  (for _ (range (+ (`KismetMathLibrary.Min` (`self.GetPoolSize`) (`self.EnemyMaxCount`)) 1))
    (bind _enemy_class (`self.GetEnemyFromPool`))
    (`/Game/StudentWork/Blueprints/Enemies/BP_Spawner.AddEnemyToQueue` (`KismetArrayLibrary.Array_Random` (`self.Spawners`)) _enemy_class)))

(fn `UserConstructionScript`)