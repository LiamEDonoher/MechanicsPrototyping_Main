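; BP_Enemy_Chaser is an enemy that chases TargetPlayer and fires projectiles.
; Move issues AIMoveTo toward TargetPlayer and zeroes the player's rotation from its Then output, while the IsValid check has empty branches.
; Attack spawns BP_Enemy_Projectile at the FirePoint location and rotation, storing it in ShootTimer despite that variable's name.
; Nothing in this graph calls Move or Attack, and the construction script only runs the parent's.
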(event `self.Move`
  (bind _targetplayer (`self.TargetPlayer`))
  ;[1 0 0 0.5] Comment
  (`/Engine/EditorBlueprintResources/StandardMacros.IsValid` _targetplayer
    (:`Is Valid`
      _)
    (:`Is Not Valid`
      _))
  (`|AIMoveTo` self (0.0 0.0 0.0) _targetplayer
    (:`then`
      (`self.K2_SetActorRotation` :`self` (`self.TargetPlayer`)))))

(event `self.Attack`
  (bind _firepoint (`self.FirePoint`))
  ; Attacking
  (bind _returnvalue (`|SpawnActorFromClass` "/Game/StudentWork/Blueprints/Projectiles/BP_Enemy_Projectile.BP_Enemy_Projectile_C" (`KismetMathLibrary.MakeTransform` (`SceneComponent.K2_GetComponentLocation` _firepoint) (`SceneComponent.K2_GetComponentRotation` _firepoint)) "Undefined" "MultiplyWithRoot" null null))
  (set `self.ShootTimer` _returnvalue))

(fn `UserConstructionScript`
  (`parent.UserConstructionScript`))