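; BP_Spawner is an enemy spawn point that spawns queued enemy classes at its own transform.
; AddEnemyToQueue appends a class and calls SpawnEnemy immediately unless a BP_Enemy_Chaser overlaps its sphere.
; SpawnEnemy spawns the first entry, removes it, and re-arms a timer on itself to drain the queue at intervals.
; Spawned enemies' destruction is bound to an event, and OnEnemyDefeated notifies the BP_WaveSpawner game mode.
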(event `OnEnemyDefeated`
  (params (DestroyedActor :type "Actor Object Reference"))
  (bind _asbp_wave_spawner (cast `/Game/StudentWork/Blueprints/Misc/BP_WaveSpawner` (`GameplayStatics.GetGameMode`)))
  (`self.OnEnemyDefeated` _asbp_wave_spawner))

(fn `AddEnemyToQueue`
  (params (Enemy :type "/Game/StudentWork/Blueprints/Enemies/BP_Enemy_Chaser Class Reference"))
  ;[1 0.8294 0] Adds enemy types to queue
  (`KismetArrayLibrary.Array_Add` (`self.EnemyQueue`) Enemy)
  ;[1 0.8294 0] Spawning Enemy
  (if (not (`KismetArrayLibrary.Array_IsValidIndex` (`PrimitiveComponent.GetOverlappingActors` (`self.Sphere`) "/Game/StudentWork/Blueprints/Enemies/BP_Enemy_Chaser.BP_Enemy_Chaser_C")))
    (`self.SpawnEnemy`)))

(fn `SpawnEnemy`
  (returns (Success :type Boolean))
  (if (`KismetArrayLibrary.Array_IsValidIndex` (`self.EnemyQueue`))
    (bind _returnvalue (`|SpawnActorFromClass` (`|GetArrayItem` (`self.EnemyQueue`)) (`self.GetTransform`) "Undefined" "MultiplyWithRoot" null null))
    (add `self.OnDestroyed` _returnvalue (`|CreateDelegate` :!event `OnEnemyDefeated`))
    (`KismetArrayLibrary.Array_Remove` (`self.EnemyQueue`))
    (`KismetSystemLibrary.K2_SetTimer` null "SpawnEnemy" 2.0)
    (return true)
    (else
      (return false))))

(fn `UserConstructionScript`)