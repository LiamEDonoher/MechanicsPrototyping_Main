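; Base enemy character Blueprint that detects the player and provides shared health and death handling.
; When the player enters AlertRadius, it stores the target and starts looping Move and Attack timers, whose events are empty here.
; Damage reduces clamped health; at zero it triggers an explosion effect and death sound, disables collision and movement, hides EnemyBase, then destroys the actor after a short delay.
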(event `self.AlertRadius.OnComponentBeginOverlap`
  (params (OverlappedComponent :type "PrimitiveComponent Object Reference") (OtherActor :type "Actor Object Reference") (OtherComp :type "PrimitiveComponent Object Reference") (OtherBodyIndex :type Integer) (bFromSweep :type Boolean) (SweepResult :type "HitResult Structure (by ref)"))
  ;[0.6172 0 0.01096] Detecting Player
  (bind _asbp_player_character (cast `/Game/Blueprints/BP_PlayerCharacter` OtherActor))
  (set `self.TargetPlayer` _asbp_player_character)
  (`self.StartMovementTimer`)
  (`self.StartAttackTimer`))

(event `StartMovementTimer`
  ;[0.6172 0 0.01096] Movement Timer
  (bind _returnvalue (`KismetSystemLibrary.K2_SetTimerDelegate` (delegate `Move`) (`self.Time`) true))
  (set `self.Movement Timer Cooldown` _returnvalue))

(event `Move`
  ;[0.6172 0 0.01096] Movement Timer
)

(event `self.ReceiveAnyDamage`
  (params (Damage :type "Float (single-precision)") (DamageType :type "DamageType Object Reference") (InstigatedBy :type "Controller Object Reference") (DamageCauser :type "Actor Object Reference"))
  ;[0.2187 1 0 0.5] Damage
  (set `self.CurrentHealth` (`KismetMathLibrary.FClamp` (- (`self.CurrentHealth`) Damage) 0.0 (`self.MaxHealth`)))
  (if (<= (`self.CurrentHealth`) 0.0)
    (`ActorComponent.Activate` (`self.NS_Explosion`) false)
    (`GameplayStatics.PlaySoundAtLocation` "/Game/StudentWork/Sounds/EnemyDeath.EnemyDeath" (0.0 0.0 0.0) (struct) 1.0 1.0 0.0 null null null null)
    (`PrimitiveComponent.SetCollisionEnabled` (`self.AlertRadius`) "NoCollision")
    (`PrimitiveComponent.SetCollisionEnabled` (`self.CapsuleComponent`) "NoCollision")
    (`SceneComponent.SetHiddenInGame` (`self.EnemyBase`) true false)
    (`CharacterMovementComponent.DisableMovement` (`self.CharacterMovement`))
    (`KismetSystemLibrary.Delay` 2.0)
    (`self.K2_DestroyActor`)))

(event `StartAttackTimer`
  ;[0.6172 0 0.01096] Attack Timer
  (bind _returnvalue (`KismetSystemLibrary.K2_SetTimerDelegate` (delegate `Attack`) (`self.AttackTimer`) true))
  (set `self.Attack Timer Cooldown` _returnvalue))

(event `Attack`
  ;[0.6172 0 0.01096] Attack Timer
)

(fn `UserConstructionScript`)