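; BP_TerminatorBoss is a boss enemy that pursues a target player and fires twin projectiles.
; Move issues an AIMoveTo toward TargetPlayer and zeroes that player's rotation, not the boss's, from the node's Then pin.
; Attack plays a fire sound and spawns enlarged BP_Enemy_Projectiles at LeftArrow and RightArrow with random positional jitter.
; BeginPlay is empty, and nothing in this file triggers Move or Attack.
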(event `self.Move`
  (bind _targetplayer (`self.TargetPlayer`))
  ;[1 0.003396 0] Moving
  (`/Engine/EditorBlueprintResources/StandardMacros.IsValid` _targetplayer
    (:`Is Valid`
      _)
    (:`Is Not Valid`
      _))
  (`|AIMoveTo` self (0.0 0.0 0.0) _targetplayer
    (:`then`
      (`self.K2_SetActorRotation` :`self` (`self.TargetPlayer`)))))

(event `self.ReceiveBeginPlay`
  ;[1 0.8294 0] Setup Variables
)

(event `self.Attack`
  (bind _returnvalue (`KismetMathLibrary.RandomFloatInRange` -20.0 20.0))
  (bind _returnvalue_2 (`KismetMathLibrary.RandomFloatInRange` -20.0 20.0))
  (bind _right_arrow (`self.Right_Arrow`))
  (bind _left_arrow (`self.Left_Arrow`))
  (bind (_returnvalue_x _returnvalue_y _returnvalue_z) (`KismetMathLibrary.BreakVector` (`SceneComponent.K2_GetComponentLocation` _right_arrow)))
  (bind (_returnvalue_x_2 _returnvalue_y_2 _returnvalue_z_2) (`KismetMathLibrary.BreakVector` (`SceneComponent.K2_GetComponentLocation` _left_arrow)))
  ;[1 0.003396 0] Attacking
  (`GameplayStatics.PlaySoundAtLocation` "/Game/StudentWork/Sounds/AUD_DefaultFire.AUD_DefaultFire" (`SceneComponent.K2_GetComponentLocation` (`self.FirePoint`)) (struct) 1.0 1.0 0.0 null null null null)
  (`|SpawnActorFromClass` "/Game/StudentWork/Blueprints/Projectiles/BP_Enemy_Projectile.BP_Enemy_Projectile_C" (`KismetMathLibrary.MakeTransform` (`KismetMathLibrary.MakeVector` (+ _returnvalue_x_2 _returnvalue_2) (+ _returnvalue_y_2 _returnvalue_2) (+ _returnvalue_z_2 _returnvalue_2)) (`SceneComponent.K2_GetComponentRotation` _left_arrow) (3.0 3.0 3.0)) "Undefined" "MultiplyWithRoot" null null)
  (bind _returnvalue_3 (`|SpawnActorFromClass` "/Game/StudentWork/Blueprints/Projectiles/BP_Enemy_Projectile.BP_Enemy_Projectile_C" (`KismetMathLibrary.MakeTransform` (`KismetMathLibrary.MakeVector` (+ _returnvalue_x _returnvalue) (+ _returnvalue_y _returnvalue) (+ _returnvalue_z _returnvalue)) (`SceneComponent.K2_GetComponentRotation` _right_arrow) (3.0 3.0 3.0)) "Undefined" "MultiplyWithRoot" null null))
  (set `self.ShootTimer` _returnvalue_3))

(fn `UserConstructionScript`
  (`parent.UserConstructionScript`))