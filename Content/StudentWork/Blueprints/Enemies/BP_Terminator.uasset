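; BP_Terminator is an enemy that continuously fires projectiles from two alternating muzzle points.
; BeginPlay fires once immediately, then starts a looping one-second timer on FireProjectile and stores its handle.
; A FlipFlop alternates each BP_Enemy_Projectile spawn between the world transforms of LeftArrow and RightArrow, with no aiming logic.
; The Hit event only prints a debug string.
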(event `self.ReceiveBeginPlay`
  (`self.Fire Projectile`)
  (bind _returnvalue (`KismetSystemLibrary.K2_SetTimerDelegate` (delegate `Fire Projectile`) 1.0 true))
  (set `self.Fire Timer` _returnvalue))

(event `Fire Projectile`
  (bind _right_arrow (`self.Right_Arrow`))
  (bind _left_arrow (`self.Left_Arrow`))
  (`/Engine/EditorBlueprintResources/StandardMacros.FlipFlop`
    (:`A`
      (`|SpawnActorFromClass` "/Game/StudentWork/Blueprints/Projectiles/BP_Enemy_Projectile.BP_Enemy_Projectile_C" (`KismetMathLibrary.MakeTransform` (`SceneComponent.K2_GetComponentLocation` _left_arrow) (`SceneComponent.K2_GetComponentRotation` _left_arrow)) "Undefined" "MultiplyWithRoot" null null))
    (:`B`
      (`|SpawnActorFromClass` "/Game/StudentWork/Blueprints/Projectiles/BP_Enemy_Projectile.BP_Enemy_Projectile_C" (`KismetMathLibrary.MakeTransform` (`SceneComponent.K2_GetComponentLocation` _right_arrow) (`SceneComponent.K2_GetComponentRotation` _right_arrow)) "Undefined" "MultiplyWithRoot" null null))))

(event `self.ReceiveHit`
  (params (MyComp :type "PrimitiveComponent Object Reference") (Other :type "Actor Object Reference") (OtherComp :type "PrimitiveComponent Object Reference") (bSelfMoved :type Boolean) (HitLocation :type "Vector Structure") (HitNormal :type "Vector Structure") (NormalImpulse :type "Vector Structure") (Hit :type "HitResult Structure (by ref)"))
  (`KismetSystemLibrary.PrintString` "Hit"))

(fn `UserConstructionScript`)