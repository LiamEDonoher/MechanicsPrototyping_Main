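; Enemy Blueprint that wanders randomly, occasionally moves toward the player and fires homing projectiles.
; Move alternates through a FlipFlop between a low-chance AI move to TargetPlayer and a move to a random reachable nearby point.
; Attack spawns BP_EnemyHoming at FirePoint with a sound, clears ShootTimer and sets the player's capsule as homing target.
; Nothing in this graph calls Move or Attack or sets TargetPlayer.
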(event `self.Move`
  ;[1 0 0 0.5] Movement
  (`/Engine/EditorBlueprintResources/StandardMacros.FlipFlop`
    (:`A`
      (bind _output_get (set `self.AttackChance` (`KismetMathLibrary.RandomInteger` 5)))
      (if (>= _output_get 4)
        (`|AIMoveTo` self (0.0 0.0 0.0) (`self.TargetPlayer`))))
    (:`B`
      (`|AIMoveTo` self (`NavigationSystemV1.K2_GetRandomReachablePointInRadius` (`self.K2_GetActorLocation`) 600.0 null null) null))))

(event `self.Attack`
  (bind _firepoint (`self.FirePoint`))
  (bind _capsulecomponent (`Character.CapsuleComponent` (`self.TargetPlayer`)))
  ;[1 0 0 0.5] Attacking
  (bind _returnvalue (`|SpawnActorFromClass` "/Game/StudentWork/Blueprints/Projectiles/BP_EnemyHoming.BP_EnemyHoming_C" (`KismetMathLibrary.MakeTransform` (`SceneComponent.K2_GetComponentLocation` _firepoint) (`SceneComponent.K2_GetComponentRotation` _firepoint)) "Undefined" "MultiplyWithRoot" null null))
  (`GameplayStatics.PlaySoundAtLocation` "/Game/StudentWork/Sounds/SmallWeaponFire.SmallWeaponFire" (`SceneComponent.K2_GetComponentLocation` (`self.FirePoint`)) (struct) 1.0 1.0 0.0 null null null null)
  (set `self.ShootTimer` null)
  (`/Engine/EditorBlueprintResources/StandardMacros.IsValid` _capsulecomponent
    (:`Is Valid`
      (set `ProjectileMovementComponent.HomingTargetComponent` _capsulecomponent (`/Game/StudentWork/Blueprints/Projectiles/BP_EnemyHoming.ProjectileMovement` _returnvalue)))))

(fn `UserConstructionScript`
  (`parent.UserConstructionScript`))