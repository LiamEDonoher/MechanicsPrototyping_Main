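; BP_Target is an explosive barrel target that detonates the first time it takes any damage.
; A DoOnce starts a timeline that flashes the barrel through a dynamic material created in the construction script.
; When the flash ends, it plays a sound at world origin, damages sphere-trace hits around itself, activates Niagara and destroys itself after a short delay.
; This area damage can chain-detonate nearby barrels.
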(event `self.ReceiveAnyDamage`
  (params (Damage :type "Float (single-precision)") (DamageType :type "DamageType Object Reference") (InstigatedBy :type "Controller Object Reference") (DamageCauser :type "Actor Object Reference"))
  (bind _returnvalue (`self.K2_GetActorLocation`))
  (`/Engine/EditorBlueprintResources/StandardMacros.DoOnce` false
    (:`Completed`
      ;[1 0.7295 0 0.5] Flash
      (bind (_direction _flash) (`Timeline|FlashTimeline` :!via `PlayFromStart`)
        (:`Update`
          (`MaterialInstanceDynamic.SetScalarParameterValue` (`self.FlashMaterial`) "FlashLerp" _flash))
        (:`Finished`
          (`GameplayStatics.PlaySoundAtLocation` "/Game/StudentWork/Sounds/AUD_Explosion.AUD_Explosion" (0.0 0.0 0.0) (struct) 1.0 1.0 0.0 null null null null)
          ;[0.05285 1 0 0.5] Damage Others
          (bind _outhits (`KismetSystemLibrary.SphereTraceMultiForObjects` _returnvalue _returnvalue 500.0 (`self.Object Types`)))
          (for _array_element _outhits
            (`GameplayStatics.ApplyDamage` (`.HitActor` (`GameplayStatics.BreakHitResult` _array_element)) 50.0))
          (`ActorComponent.Activate` (`self.NS_Explosion`) false)
          (`KismetSystemLibrary.Delay` 0.3)
          (`self.K2_DestroyActor`))))))

(fn `UserConstructionScript`
  (bind _returnvalue (`PrimitiveComponent.CreateDynamicMaterialInstance` (`self.SM_Barrel`) 0 "/Game/StudentWork/Materials/M_ExplosiveFlash.M_ExplosiveFlash" "FlashMaterial"))
  (set `self.FlashMaterial` _returnvalue))