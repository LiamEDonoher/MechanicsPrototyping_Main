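; BP_BigHitta_Weapon is a tank weapon that fires a BigHitta projectile when triggered.
; If no cooldown is active, it spawns the projectile at the owning tank's direction arrow, matching its facing, and plays the BigHitta sound at that spot.
; It then sets a cooldown flag and starts a short timer whose event clears the flag so the weapon can fire again.
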(event `self.Triggered`
  (bind (_returnvalue_location _returnvalue_rotation) (`KismetMathLibrary.BreakTransform` (`SceneComponent.K2_GetComponentToWorld` (`/Game/Blueprints/BP_PlayerCharacter.DirectionArrow` (`self.MyTank`)))))
  (if (not (`self.IsCooldownActive?`))
    (bind _returnvalue (`|SpawnActorFromClass` "/Game/StudentWork/Blueprints/Projectiles/BP_BigHitta_Projectile.BP_BigHitta_Projectile_C" (`KismetMathLibrary.MakeTransform` _returnvalue_location _returnvalue_rotation) "Undefined" "MultiplyWithRoot" null null))
    (`GameplayStatics.PlaySoundAtLocation` "/Game/StudentWork/Sounds/BigHitta.BigHitta" (`self.K2_GetActorLocation` _returnvalue) (struct) 1.0 1.0 0.0 null null null null)
    (set `self.IsCooldownActive?` true)
    (`KismetSystemLibrary.K2_SetTimerDelegate` (delegate `EndCooldown`) 3.0)))

(event `EndCooldown`
  (set `self.IsCooldownActive?` false))

(fn `UserConstructionScript`
  (`parent.UserConstructionScript`))