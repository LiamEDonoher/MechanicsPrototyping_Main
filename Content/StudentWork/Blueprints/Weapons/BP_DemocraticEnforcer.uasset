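; BP_DemocraticEnforcer is a tank weapon that fires a projectile when triggered.
; Triggered spawns a BP_DemocraticEnforcer_Projectile at the world location and rotation of the owning tank's DirectionArrow.
; A boolean cooldown flag blocks further shots until a short timer event clears it.
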(event `self.Triggered`
  (bind (_returnvalue_location _returnvalue_rotation) (`KismetMathLibrary.BreakTransform` (`SceneComponent.K2_GetComponentToWorld` (`/Game/Blueprints/BP_PlayerCharacter.DirectionArrow` (`self.MyTank`)))))
  (if (not (`self.IsCooldownActive?`))
    (`|SpawnActorFromClass` "/Game/StudentWork/Blueprints/Projectiles/BP_DemocraticEnforcer_Projectile.BP_DemocraticEnforcer_Projectile_C" (`KismetMathLibrary.MakeTransform` _returnvalue_location _returnvalue_rotation) "Undefined" "MultiplyWithRoot" null null)
    (set `self.IsCooldownActive?` true)
    (`KismetSystemLibrary.K2_SetTimerDelegate` (delegate `CustomEvent`) 1.5)))

(event `CustomEvent`
  (set `self.IsCooldownActive?` false))

(fn `UserConstructionScript`
  (`parent.UserConstructionScript`))